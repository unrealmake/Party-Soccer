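; AI-controlled character that chases BP_Ball, occasionally rolling to dash when far from it or punching when close.
; BeginPlay sets walk speed and blends physics into the mesh through PhysicalAnimation, simulating bodies below a chosen bone.
; Tick calls ReLoad, then picks by distance and random roll between Walking toward the ball, Punch, or an inline timed speed-boost dash.
; The separate Dash function duplicates that boost without a connected speed reset and is not called here.
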(event EventBeginPlay
  (bind _body_name (Variables|Default|GetBody%20Name))
  (|CallParentFunction)
  (Variables|/Script/Engine.CharacterMovementComponent|SetMaxWalkSpeed (Variables|Character|GetCharacterMovement) 5e+02)
  (Variables|Default|SetJumpMaxCount 1)
  ;[1 1 1] 렉돌 구현
  (Class|PhysicalAnimationComponent|SetSkeletalMeshComponent (Variables|Default|GetPhysicalAnimation) (Variables|Character|GetMesh))
  (Class|PhysicalAnimationComponent|ApplyPhysicalAnimationSettingsBelow (Variables|Default|GetPhysicalAnimation) _body_name (Utilities|Struct|MakePhysicalAnimationData true 1e+03 1e+02 1e+02 1e+02 1e+02 8e+01) true)
  (Class|SkeletalMeshComponent|SetAllBodiesBelowSimulatePhysics (Variables|Character|GetMesh) _body_name true false))

(event Collision|EventActorBeginOverlap
  (params (OtherActor :type Actor%20Object%20Reference))
  (|CallParentFunction OtherActor) ; This node is disabled and will not be called.\nDrag off pins to build functionality.
)

(event EventTick
  (params (DeltaSeconds :type Float%20%28single-precision%29))
  (|CallParentFunction DeltaSeconds)
  (CallFunction|ReLoad)
  (bind _returnvalue (Actor|GetActorOfClass "/Game/_Main/Blueprints/BP_Ball.BP_Ball_C"))
  (if (> (Math|Vector|VectorLength (- (Transformation|GetActorLocation _returnvalue) (Transformation|GetActorLocation))) 5e+02)
    (if (== (Math|Random|RandomInteger 150) 100)
      (Variables|/Script/Engine.CharacterMovementComponent|SetMaxWalkSpeed (Variables|Character|GetCharacterMovement) 1e+03)
      (Animation|PlayAnimMontage "/Game/ControlRig/Characters/Mannequins/Animations/RollAnim_Montage.RollAnim_Montage" 3.0 "None")
      (Utilities|FlowControl|Delay 0.5)
      (Variables|/Script/Engine.CharacterMovementComponent|SetMaxWalkSpeed (Variables|Character|GetCharacterMovement) 5e+02)
      (else
        (CallFunction|Walking)))
    (elif (== (Math|Random|RandomInteger 30) 15)
      (CallFunction|Punch)
      (else
        (CallFunction|Walking)))))

(fn ConstructionScript
  (|CallParentFunction))

(fn Walking
  (bind _returnvalue (Actor|GetActorOfClass "/Game/_Main/Blueprints/BP_Ball.BP_Ball_C"))
  (Pawn|Input|AddMovementInput (- (Transformation|GetActorLocation _returnvalue) (Transformation|GetActorLocation)) 1.0 false))

(fn Dash
  (Variables|/Script/Engine.CharacterMovementComponent|SetMaxWalkSpeed (Variables|Character|GetCharacterMovement) 1e+03)
  (Animation|PlayAnimMontage "/Game/ControlRig/Characters/Mannequins/Animations/RollAnim_Montage.RollAnim_Montage" 3.0 "None"))
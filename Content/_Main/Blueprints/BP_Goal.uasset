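; BP_Goal is a goal actor that counts a score when a BP_Ball hits its Cube and then restarts with a fresh ball.
; A hit destroys the ball and swaps the Cube material, then after a short delay shows BP_Widget, sets IsLoading on BP_MainCharacter and spawns a new ball at world origin.
; After a second delay it sets the black unlit material and removes all widgets.
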(event OnComponentHit(Cube)
  (params (HitComponent :type Primitive%20Component%20Object%20Reference) (OtherActor :type Actor%20Object%20Reference) (OtherComp :type Primitive%20Component%20Object%20Reference) (NormalImpulse :type Vector :default "0, 0, 0") (Hit :type Hit%20Result%20Structure%20%28by%20ref%29))
  (bind _asbp_ball (Utilities|Casting|CastToBP_Ball OtherActor))
  (Variables|Default|SetScore (+ (Variables|Default|GetScore) 1))
  (Actor|DestroyActor _asbp_ball)
  (Rendering|Material|SetMaterial (Variables|Default|GetCube) 0 "/Engine/EngineDebugMaterials/BoneWeightMaterial.BoneWeightMaterial")
  (Utilities|FlowControl|Delay 0.2)
  (bind _returnvalue (UserInterface|CreateWidget "/Game/_Main/Blueprints/BP_Widget.BP_Widget_C"))
  (UserInterface|Viewport|AddtoViewport _returnvalue 0)
  (bind _returnvalue_2 (Actor|GetActorOfClass "/Game/_Main/Blueprints/BP_MainCharacter.BP_MainCharacter_C"))
  (Variables|/Game/_Main/Blueprints/BP_MainCharacter.BP_MainCharacter_C|SetisLoading _returnvalue_2 true)
  (Game|SpawnActorfromClass "/Game/_Main/Blueprints/BP_Ball.BP_Ball_C" (Math|Conversions|ToTransform(Vector) (Math|Vector|MakeVector 0.0 0.0 0.0)) "Undefined" "MultiplyWithRoot" 0 0)
  (Utilities|FlowControl|Delay 2.0)
  (Rendering|Material|SetMaterial (Variables|Default|GetCube) 0 "/Engine/EngineDebugMaterials/BlackUnlitMaterial.BlackUnlitMaterial")
  (Viewport|RemoveAllWidgets))

(event EventBeginPlay)

(event Collision|EventActorBeginOverlap
  (params (OtherActor :type Actor%20Object%20Reference)))

(event EventTick
  (params (DeltaSeconds :type Float%20%28single-precision%29)))

(fn ConstructionScript)
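; BP_MainCharacter is the player character Blueprint, handling movement setup and mouse camera rotation.
; On BeginPlay it applies MoveSpeed as walk speed, widens the camera pitch limits to a full turn either way, allows a single jump and registers the IMC_Player Enhanced Input mapping context.
; The IA_CameraRotaion action feeds its X and Y values into controller yaw and pitch.
; The graph contains no move or jump input handlers.
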(event Input|EnhancedActionEvents|EnhancedInputActionIA_CameraRotaion
  (params (ActionValue :type Vector%202D%20Structure) (ElapsedSeconds :type Float%20%28double-precision%29) (TriggeredSeconds :type Float%20%28double-precision%29) (InputAction :type Input%20Action%20Object%20Reference :default "/Game/Input/IA_CameraRotaion.IA_CameraRotaion"))
  ;[1 1 1] 마우스 카메라 이동
  (Pawn|Input|AddControllerYawInput (.x ActionValue))
  (Pawn|Input|AddControllerPitchInput (.y ActionValue)))

(event EventBeginPlay
  (bind _returnvalue (Game|GetPlayerCameraManager 0))
  ;[1 1 1] 걷는 속도 조정
  (Variables|/Script/Engine.CharacterMovementComponent|SetMaxWalkSpeed (Variables|Character|GetCharacterMovement) (Variables|Default|GetMoveSpeed))
  ;[1 1 1] 카메라 상/하 각도 제한
  (Variables|/Script/Engine.PlayerCameraManager|SetViewPitchMin _returnvalue -3.6e+02)
  (Variables|/Script/Engine.PlayerCameraManager|SetViewPitchMax _returnvalue 3.6e+02)
  ;[1 1 1] 점프는 1번만 가능
  (Variables|Default|SetJumpMaxCount 1)
  ;[1 1 1] Input 적용
  (bind _asplayer_controller (Utilities|Casting|CastToPlayerController (Pawn|GetController)))
  (Input|AddMappingContext (PlayerController|LocalPlayerSubsystems|GetEnhancedInputLocalPlayerSubsystem _asplayer_controller) "/Game/Input/IMC_Player.IMC_Player" 0 "(bIgnoreAllPressedKeysUntilRelease=True,bForceImmediately=False,bNotifyUserSettings=False)"))

(event Collision|EventActorBeginOverlap
  (params (OtherActor :type Actor%20Object%20Reference)))

(event EventTick
  (params (DeltaSeconds :type Float%20%28single-precision%29)))

(fn ConstructionScript)